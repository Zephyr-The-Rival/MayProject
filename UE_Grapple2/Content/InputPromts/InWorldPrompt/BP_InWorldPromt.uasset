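; BP_InWorldPromt shows an input prompt in the world as a textured image plane for a given action, matching the player's current input device.
; The construction script creates a dynamic instance of M_InputPrompt, then sets its texture and tint.
; On BeginPlay it binds to BP_GrapplePlayerController's device-switch event, refreshing the gamepad or mouse-and-keyboard texture, with optional overrides for each.
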(event `self.ReceiveBeginPlay`
  (`|ExecutionSequence`
    (:`then_0`
      (bind _asbp_grapple_player_controller (cast `/Game/Grapple/Player/BP_GrapplePlayerController` (`GameplayStatics.GetPlayerController` 0)))
      (add `/Game/Grapple/Player/BP_GrapplePlayerController.OnInputDeviceSwitched` _asbp_grapple_player_controller (`|CreateDelegate` :!event `OnDeviceChanged`))
      (set `self.Gamepad` (`/Game/Grapple/Player/BP_GrapplePlayerController.IsUsingGamepad` _asbp_grapple_player_controller)))
    (:`then_1`
      (`self.InititializePromptWidget`))))

(event `InititializePromptWidget`
  (bind _texture (`/Game/InputPromts/BP_PromptFunctions.GetPromptTexture` (`self.Action`) (`self.OverrideGamepadTexture`) (`self.OverrideMaKTexture`) (`self.Gamepad`)))
  (`MaterialInstanceDynamic.SetTextureParameterValue` (`self.InputPromptMaterial`) "Texture" _texture))

(event `SetTint`
  (bind _inputpromptmaterial (`self.InputPromptMaterial`))
  (`/Engine/EditorBlueprintResources/StandardMacros.IsValid` _inputpromptmaterial
    (:`Is Valid`
      (`MaterialInstanceDynamic.SetVectorParameterValue` _inputpromptmaterial "Color" (`self.Color`)))))

(event `OnDeviceChanged`
  (params (Gamepad :type Boolean))
  (set `self.Gamepad` Gamepad)
  (`self.InititializePromptWidget`))

(fn `UserConstructionScript`
  (`|ExecutionSequence`
    (:`then_0`
      (bind _returnvalue (`PrimitiveComponent.CreateDynamicMaterialInstance` (`self.ImagePlane`) 0 "/Game/InputPromts/InWorldPrompt/M_InputPrompt.M_InputPrompt" "None"))
      (set `self.InputPromptMaterial` _returnvalue))
    (:`then_1`
      (`|ExecutionSequence`
        (:`then_0`
          (`self.InititializePromptWidget`))
        (:`then_1`
          (`self.SetTint`))))))