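; BP_InWorldPromt_WithText is an in-world input prompt variant that adds left and right text labels.
; The construction script runs the parent's setup, then SetText copies TextLeft and TextRight into the two text render components.
; SetTint extends the parent's tinting by applying the same Color to both labels, converted without sRGB.
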(event `SetText`
  (`|ExecutionSequence`
    (:`then_0`
      (`TextRenderComponent.K2_SetText` (`self.Text_L`) (`self.Text_Left`)))
    (:`then_1`
      (`TextRenderComponent.K2_SetText` (`self.Text_R`) (`self.Text_Right`)))))

(event `self.SetTint`
  (`parent.SetTint`)
  (`|ExecutionSequence`
    (:`then_0`
      (`TextRenderComponent.SetTextRenderColor` (`self.Text_L`) (`KismetMathLibrary.Conv_LinearColorToColor` (`self.Color`) false)))
    (:`then_1`
      (`TextRenderComponent.SetTextRenderColor` (`self.Text_R`) (`KismetMathLibrary.Conv_LinearColorToColor` (`self.Color`) false)))))

(fn `UserConstructionScript`
  (`parent.UserConstructionScript`)
  (`self.SetText`))