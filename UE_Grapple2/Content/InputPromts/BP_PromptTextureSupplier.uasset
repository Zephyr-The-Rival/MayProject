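; BP_PromptTextureSupplier supplies input prompt textures for a given action and mapping context, for gamepad or mouse and keyboard.
; GetActionTexture resolves the bound key through GetKeyFromAction, then scans the device's data table row by row for that key.
; It synchronously loads the matching row's texture reference, using the V2 variant when alternative gamepad keys are enabled, and returns it as a Texture2D.
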(fn `GetActionTexture`
  (params (Action :type "InputAction Object Reference") (MappingContext :type "InputMappingContext Object Reference") (Gamepad :type Boolean))
  (returns (ReturnValue :type "Texture2D Object Reference"))
  (locals (KeyToFind :type "Key Structure" :default "None") (TableToSearch :type "DataTable Object Reference" :default "/Script/Engine.DataTable'/Game/InputPromts/TextureTable_Gamepad.TextureTable_Gamepad'") (ReferenceToLoad :type "Texture2D Soft Object Reference") (Local_Gamepad :type Boolean))
  (set `local.Local_Gamepad` Gamepad)
  (`|ExecutionSequence`
    (:`then_0`
      (bind _key (`/Game/InputPromts/BP_PromptFunctions.GetKeyFromAction` Action MappingContext (`local.Local_Gamepad`)))
      (set `local.KeyToFind` _key))
    (:`then_1`
      (if (`local.Local_Gamepad`)
        (set `local.TableToSearch` "/Game/InputPromts/TextureTable_Gamepad.TextureTable_Gamepad") ; gamepad texture table
        (else
          (set `local.TableToSearch` "/Game/InputPromts/TextureTable_MaK.TextureTable_MaK") ; mouse and keyboard texture table
        )))
    (:`then_2`
      (bind _outrownames (`DataTableFunctionLibrary.GetDataTableRowNames` (`local.TableToSearch`)))
      (for _array_element _outrownames
        (bind _returnvalue (`|GetDataTableRow` (`local.TableToSearch`) _array_element)
          (:`then`
            (bind (_key_2 _textureassetref _texturev2assetref) (break `/Game/InputPromts/InputPromtTexture` _returnvalue))
            (if (== _key_2 (`local.KeyToFind`))
              (`|ExecutionSequence`
                (:`then_0`
                  (if (and (`local.Local_Gamepad`) (`self.AlternativeGamepadKeys`))
                    (set `local.ReferenceToLoad` _texturev2assetref)
                    (else
                      (set `local.ReferenceToLoad` _textureassetref))))
                (:`then_1`
                  (bind _returnvalue_2 (`KismetSystemLibrary.LoadAsset_Blocking` (`local.ReferenceToLoad`)))
                  (bind _astexture_2d (cast `Texture2D` _returnvalue_2))
                  (return _astexture_2d))))))))))

(fn `UserConstructionScript`)