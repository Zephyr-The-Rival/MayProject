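; BP_PromptFunctions is a set of helper functions that resolve which input prompt texture to show for an input action.
; GetPromptTexture returns the gamepad or mouse-and-keyboard override if supplied, otherwise asks the level's BP_PromptTextureSupplier actor using the PlayerCharacterInput context.
; Distinct placeholder textures flag a missing action, supplier or texture.
; GetKeyFromAction separately finds an action's first gamepad or non-gamepad key in a mapping context.
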(fn `GetKeyFromAction`
  (params (Action :type "Object Object Reference") (MappingContext :type "InputMappingContext Object Reference") (LookingForGamepadKey :type Boolean))
  (returns (Key :type "Key Structure"))
  (for _array_element (`InputMappingContext.Mappings` MappingContext)
    (bind (_triggers _modifiers _action _key) (break `EnhancedActionKeyMapping` _array_element))
    (if (and (== (`KismetInputLibrary.Key_IsGamepadKey` _key) LookingForGamepadKey) (== Action _action))
      (return _key))))

(fn `GetPromptTexture`
  (params (Action :type "InputAction Object Reference") (OverrideGamepadTexture :type "Texture2D Object Reference") (OverrideMaKTexture :type "Texture2D Object Reference") (Gamepad :type Boolean))
  (returns (Texture :type "Texture2D Object Reference"))
  (locals (Local_OverrideGamepadTexture :type "Texture2D Object Reference") (Local_OverrideMaKTexture :type "Texture2D Object Reference") (Local_Gamepad :type Boolean))
  (`|ExecutionSequence`
    (:`then_0`
      (set `local.Local_OverrideGamepadTexture` OverrideGamepadTexture)
      (set `local.Local_OverrideMaKTexture` OverrideMaKTexture)
      (set `local.Local_Gamepad` Gamepad))
    (:`then_1`
      (`/Engine/EditorBlueprintResources/StandardMacros.IsValid` Action
        (:`Is Valid`
          (bind _returnvalue (`GameplayStatics.GetActorOfClass` (`local.__WorldContext`) "/Game/InputPromts/BP_PromptTextureSupplier.BP_PromptTextureSupplier_C"))
          (`/Engine/EditorBlueprintResources/StandardMacros.IsValid` _returnvalue
            (:`Is Valid`
              (`|ExecutionSequence`
                (:`then_0`
                  ; OverrideTextures
                  (`|ExecutionSequence`
                    (:`then_0`
                      (if (and (`KismetSystemLibrary.IsValid` (`local.Local_OverrideGamepadTexture`)) (`local.Local_Gamepad`))
                        (return (`local.Local_OverrideGamepadTexture`))))
                    (:`then_1`
                      (if (and (`KismetSystemLibrary.IsValid` (`local.Local_OverrideMaKTexture`)) (not (`local.Local_Gamepad`)))
                        (return (`local.Local_OverrideMaKTexture`))))))
                (:`then_1`
                  (bind _returnvalue_2 (`/Game/InputPromts/BP_PromptTextureSupplier.GetActionTexture` _returnvalue (`local.Action`) "/Game/Grapple/Player/Input/PlayerCharacterInput.PlayerCharacterInput" (`local.Local_Gamepad`))) ; Get texture from supplier
                  (`/Engine/EditorBlueprintResources/StandardMacros.IsValid` _returnvalue_2
                    (:`Is Valid`
                      (return _returnvalue_2))
                    (:`Is Not Valid`
                      (return "/Game/InputPromts/Textures/Errors/T_NoTextureAviable.T_NoTextureAviable"))))))
            (:`Is Not Valid`
              (return "/Game/InputPromts/Textures/Errors/T_NoTextureSupplierFound.T_NoTextureSupplierFound"))))
        (:`Is Not Valid`
          (return "/Game/InputPromts/Textures/Errors/T_NoActionSelected.T_NoActionSelected"))))))