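; A grapple object Blueprint that can be kicked and returns the velocity the kicking player should have afterwards.
; Kick broadcasts the OnKicked dispatcher with the kicker, direction and strength, leaving any reaction to bound listeners.
; It then passes direction times strength to CalculatePostKickPlayerVelocity, which halves that vector for the return value.
; The event graph and construction script add no logic beyond parent calls.
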(event `self.ReceiveTick`
  (params (DeltaSeconds :type "Float (single-precision)"))
  (`parent.ReceiveTick` DeltaSeconds))

(fn `CalculatePostKickPlayerVelocity`
  (params (OldVelocity :type "Vector Structure"))
  (returns (NewVelocity :type "Vector Structure"))
  (return (* OldVelocity (0.5 0.5 0.5))))

(fn `Kick`
  (params (TheKicker :type "/Game/Grapple/Player/BP_GrapplePlayerCharacter Object Reference") (Direction :type "Vector Structure") (Strenght :type "Float (double-precision)"))
  (returns (NewVelocity :type "Vector Structure"))
  (`self.OnKicked` TheKicker Direction Strenght)
  (bind _newvelocity (`self.CalculatePostKickPlayerVelocity` (* Direction Strenght)))
  (return _newvelocity))

(fn `UserConstructionScript`
  (`parent.UserConstructionScript`))