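; BP_KickExampleObject is an example kickable object that gets launched as a physics body when kicked.
; Its Kick override calls the parent, then turns on physics simulation for the static mesh.
; It applies linear and scaled-down angular impulses from direction times strength, both as velocity changes so mass is ignored.
; The event graph holds only disabled stubs, so all of its own behavior lives in Kick.
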(fn `Kick`
  (params (TheKicker :type "/Game/Grapple/Player/BP_GrapplePlayerCharacter Object Reference") (Direction :type "Vector Structure") (Strenght :type "Float (double-precision)"))
  (returns (PostKickPlayerVelocity :type "Vector Structure"))
  (bind _returnvalue (* Direction Strenght))
  (bind _postkickplayervelocity (`parent.Kick` TheKicker Direction Strenght))
  (`PrimitiveComponent.SetSimulatePhysics` (`self.StaticMesh`) true)
  (`PrimitiveComponent.AddImpulse` (`self.StaticMesh`) _returnvalue "None" true)
  (`PrimitiveComponent.AddAngularImpulseInDegrees` (`self.StaticMesh`) (* _returnvalue (0.2 0.2 0.2)) "None" true)
  (return _postkickplayervelocity))

(fn `UserConstructionScript`
  (`parent.UserConstructionScript`))