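; BP_SmashableWall is a grapple-object wall that shatters into physics debris when kicked.
; BeginPlay caches the pre-placed mesh pieces, and GetGrappleLocation exposes the grapple point.
; Kick destroys the intact Cube and Box, reveals the pieces with an impulse from the kicker's grapple position, spawns concrete Niagara FX, and returns a scaled kick vector.
; PostSmash removes debris and actor after a delay; the debris dust trail is unconnected.
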(event `self.ReceiveBeginPlay`
  (`parent.ReceiveBeginPlay`)
  (set `self.DebrisPieces` (`|MakeArray` (`self.5x5SMashable_SM_23_`) (`self.5x5SMashable_SM_10_`) (`self.5x5SMashable_SM_11_`) (`self.5x5SMashable_SM_12_`) (`self.5x5SMashable_SM_13_`) (`self.5x5SMashable_SM_14_`) (`self.5x5SMashable_SM_15_`) (`self.5x5SMashable_SM_16_`) (`self.5x5SMashable_SM_17_`) (`self.5x5SMashable_SM_18_`) (`self.5x5SMashable_SM_19_`) (`self.5x5SMashable_SM_2_`) (`self.5x5SMashable_SM_20_`) (`self.5x5SMashable_SM_21_`) (`self.5x5SMashable_SM_22_`) (`self.5x5SMashable_SM_1_`) (`self.5x5SMashable_SM_24_`) (`self.5x5SMashable_SM_25_`) (`self.5x5SMashable_SM_26_`) (`self.5x5SMashable_SM_27_`) (`self.5x5SMashable_SM_28_`) (`self.5x5SMashable_SM_29_`) (`self.5x5SMashable_SM_3_`) (`self.5x5SMashable_SM_30_`) (`self.5x5SMashable_SM_4_`) (`self.5x5SMashable_SM_5_`) (`self.5x5SMashable_SM_6_`) (`self.5x5SMashable_SM_7_`) (`self.5x5SMashable_SM_8_`) (`self.5x5SMashable_SM_9_`))))

(event `PostSmash`
  (`KismetSystemLibrary.Delay` 10.0)
  (`|ExecutionSequence`
    (:`then_0`
      (for _array_element (`self.DebrisPieces`)
        (`ActorComponent.K2_DestroyComponent` _array_element)))
    (:`then_1`
      (`self.K2_DestroyActor`))))

(fn `GetGrappleLocation`
  (returns (GrappleLocation :type "Vector Structure"))
  (return (`SceneComponent.K2_GetComponentLocation` (`self.GrappleLocation`))))

(fn `Kick`
  (params (TheKicker :type "/Game/Grapple/Player/BP_GrapplePlayerCharacter Object Reference") (Direction :type "Vector Structure") (Strenght :type "Float (double-precision)"))
  (returns (PostKickPlayerVelocity :type "Vector Structure"))
  (bind _returnvalue_location (`KismetMathLibrary.BreakTransform` (`SceneComponent.K2_GetComponentToWorld` (`self.GrappleLocation`))))
  (`|ExecutionSequence`
    (:`then_0`
      (`|ExecutionSequence`
        (:`then_0`
          (`ActorComponent.K2_DestroyComponent` (`self.Cube`))
          (`ActorComponent.K2_DestroyComponent` (`self.Box`)))
        (:`then_1`
          (for _array_element (`self.DebrisPieces`)
            (`SceneComponent.SetHiddenInGame` _array_element false false)
            (`PrimitiveComponent.SetSimulatePhysics` _array_element true)
            (`PrimitiveComponent.SetCollisionEnabled` _array_element "PhysicsOnly")
            (`PrimitiveComponent.AddImpulseAtLocation` _array_element (* (`local.Direction`) (`local.Strenght`) 30.0) (`/Game/Grapple/Player/GrappleTargetFinder/GrappleTargetFinder.GetGrapplePosition` (`/Game/Grapple/Player/BP_GrapplePlayerCharacter.GrappleTargetFinder` TheKicker)) "None")))
        (:`then_2`
          (`NiagaraFunctionLibrary.SpawnSystemAtLocation` "/Game/Grapple/GrappleObjects/Smashable/5x5Wall/NS_ConcreteSmash.NS_ConcreteSmash" _returnvalue_location (`KismetMathLibrary.MakeRotFromX` (`local.Direction`))))))
    (:`then_1`
      (`self.PostSmash`))
    (:`then_2`
      (return (* Direction Strenght 0.5)))))

(fn `UserConstructionScript`
  (`parent.UserConstructionScript`))