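; BP_Rocket is a player-spawned projectile that carries a child grapple object, so grapple shooters can hook onto it in flight.
; An Accelerate timeline blends velocity from the spawning player's velocity plus a small forward push up to max forward speed.
; Tick moves it with a swept offset, exploding on a blocking hit or after a fixed delay.
; Explode prints a message, interrupts any connected grapple and destroys the rocket.
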(event `self.ReceiveBeginPlay`
  (`|ExecutionSequence`
    (:`then_0`
      (`|ExecutionSequence`
        (:`then_0`
          (set `self.Velocity` (+ (`/Game/Grapple/Player/PositionBasedVelocityCalculator.GetVelocity` (`/Game/Grapple/Player/BP_GrapplePlayerCharacter.CharacterIndipendantVelocity` (`self.SpawningPlayer`))) (* (`self.GetActorForwardVector`) (50.0 50.0 50.0))))
          (set `self.TargetVelocity` (* (`self.GetActorForwardVector`) (`self.MaxSpeed`))))
        (:`then_1`
          (bind (_direction _0_to_1) (`Timeline|Accelerate` :!via `PlayFromStart`)
            (:`Update`
              (set `self.Velocity` (`KismetMathLibrary.VLerp` (+ (`/Game/Grapple/Player/PositionBasedVelocityCalculator.GetVelocity` (`/Game/Grapple/Player/BP_GrapplePlayerCharacter.CharacterIndipendantVelocity` (`self.SpawningPlayer`))) (* (`self.GetActorForwardVector`) (50.0 50.0 50.0))) (`self.TargetVelocity`) _0_to_1)))))))
    (:`then_1`
      (`KismetSystemLibrary.Delay` 5.0)
      (`self.Explode`))
    (:`then_2`
      (bind _asbp_grapple_object (cast `/Game/Grapple/GrappleObjects/BP_GrappleObject` (`ChildActorComponent.ChildActor` (`self.GrappleObject`))))
      (add `/Game/Grapple/GrappleObjects/BP_GrappleObject.OnLetGo` _asbp_grapple_object (`|CreateDelegate` :!event `LetGo`))
      (add `/Game/Grapple/GrappleObjects/BP_GrappleObject.OnHooked` _asbp_grapple_object (`|CreateDelegate` :!event `Hooked`)))))

(event `self.ReceiveTick`
  (params (DeltaSeconds :type "Float (single-precision)"))
  (bind _sweephitresult (`self.K2_AddActorWorldOffset` (* (`self.Velocity`) (`GameplayStatics.GetWorldDeltaSeconds`)) true))
  (if (`GameplayStatics.BreakHitResult` _sweephitresult)
    (`self.Explode`)))

(event `Hooked`
  (params (GrappleShooter :type "/Game/Grapple/Player/GrappleShooter/BP_GrappleShooter Object Reference"))
  (set `self.Conntected Grapple Shooter` GrappleShooter))

(event `LetGo`
  (params (GrappleShooter :type "/Game/Grapple/Player/GrappleShooter/BP_GrappleShooter Object Reference"))
  (set `self.Conntected Grapple Shooter` null))

(event `Explode`
  (bind _conntected_grapple_shooter (`self.Conntected Grapple Shooter`))
  (`|ExecutionSequence`
    (:`then_0`
      (`KismetSystemLibrary.PrintString` "Boom"))
    (:`then_1`
      (`/Engine/EditorBlueprintResources/StandardMacros.IsValid` _conntected_grapple_shooter
        (:`Is Valid`
          (`/Game/Grapple/Player/GrappleShooter/BP_GrappleShooter.InterruptGrapple` _conntected_grapple_shooter))))
    (:`then_2`
      (`self.K2_DestroyActor`))))

(fn `GetGrappleLocation`
  (returns (GrappleLocation :type "Vector Structure"))
  (return (`self.K2_GetActorLocation`)))

(fn `UserConstructionScript`)