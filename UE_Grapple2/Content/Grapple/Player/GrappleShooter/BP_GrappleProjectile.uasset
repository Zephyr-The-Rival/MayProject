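; Projectile fired by the grapple shooter that flies out, attaches to whatever it hits and signals the hit.
; Each tick it either lerps to a guaranteed target over a time scaled by distance relative to grapple range, or moves straight forward.
; Both moves sweep, so any blocker in the way becomes the attach point, with impact sound and particle burst.
; StopProjectile disables collision and movement during reel-in, leaving the return to the shooter.
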(event `self.ReceiveBeginPlay`
  (if (`self.MovingToGuaranteedHit`)
    (`|ExecutionSequence`
      (:`then_0`
        (set `self.StartPosition` (`self.K2_GetActorLocation`)))
      (:`then_1`
        (set `self.MoveTimeBasedOnDistance` (* (`KismetMathLibrary.FClamp` (/ (`KismetMathLibrary.Vector_Distance` (`self.StartPosition`) (`self.K2_GetActorLocation` (`self.ProjectileTarget`))) (`self.GrappleRange`))) (`self.ProjectileMaxMoveTime`)))))))

(event `StopProjectile`
  (`PrimitiveComponent.SetCollisionEnabled` (`self.ProjectileMesh`) "NoCollision")
  (set `self.Move` false))

(event `self.ReceiveTick`
  (params (DeltaSeconds :type "Float (single-precision)"))
  (bind _projectiletarget (`self.ProjectileTarget`))
  (if (`self.Move`)
    (if (`self.MovingToGuaranteedHit`)
      (set `self.MoveTimeCounter` (+ (`self.MoveTimeCounter`) (`GameplayStatics.GetWorldDeltaSeconds`)))
      (if (<= (`self.MoveTimeCounter`) (`self.MoveTimeBasedOnDistance`))
        (bind _sweephitresult (`self.K2_SetActorLocation` (`KismetMathLibrary.VLerp` (`self.StartPosition`) (`self.K2_GetActorLocation` (`self.ProjectileTarget`)) (/ (`self.MoveTimeCounter`) (`self.MoveTimeBasedOnDistance`))) true))
        (bind (_bblockinghit _binitialoverlap _time _distance _location _impactpoint _normal _impactnormal _physmat _hitactor _hitcomponent) (`GameplayStatics.BreakHitResult` _sweephitresult))
        (if _bblockinghit
          (`self.ProjectileHit` _hitcomponent _location))
        (else
          (`self.ProjectileHit` (`Actor.RootComponent` _projectiletarget) (`self.K2_GetActorLocation` _projectiletarget))))
      (else
        (bind _sweephitresult_2 (`self.K2_AddActorWorldOffset` (* (`self.GetActorForwardVector`) (`GameplayStatics.GetWorldDeltaSeconds`) (`self.MovingForwardSpeed`)) true))
        (bind (_bblockinghit_2 _binitialoverlap_2 _time_2 _distance_2 _location_2 _impactpoint_2 _normal_2 _impactnormal_2 _physmat_2 _hitactor_2 _hitcomponent_2) (`GameplayStatics.BreakHitResult` _sweephitresult_2))
        (if _bblockinghit_2
          (`self.ProjectileHit` _hitcomponent_2 _location_2))))))

(event `ProjectileHit`
  (params (ParentAttachComponent :type "SceneComponent Object Reference") (NewLocation :type "Vector Structure"))
  (`|ExecutionSequence`
    (:`then_0`
      (`self.K2_SetActorLocation` NewLocation)
      (set `self.Move` false)
      (`self.K2_AttachToComponent` ParentAttachComponent "None" "KeepWorld" "KeepWorld" "KeepWorld"))
    (:`then_1`
      (`self.PlayFeedback`))
    (:`then_2`
      (`self.OnProjectileHit`))))

(event `PlayFeedback`
  (`|ExecutionSequence`
    (:`then_0`
      (`GameplayStatics.PlaySound2D` "/Game/Grapple/SFX/GrapplerSoundsPack/GrappleProjectileImpact.GrappleProjectileImpact" 1.0 1.0 0.0 null null))
    (:`then_1`
      (`NiagaraFunctionLibrary.SpawnSystemAtLocation` "/Niagara/DefaultAssets/Templates/Systems/DirectionalBurstLightweight.DirectionalBurstLightweight" (`SceneComponent.K2_GetComponentLocation` (`self.ProjectileMesh`))))))

(fn `UserConstructionScript`)