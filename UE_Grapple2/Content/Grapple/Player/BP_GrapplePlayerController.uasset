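; Player controller for the Grapple game that manages input mode, input device detection and the pause menu.
; Any key press updates the gamepad flag, broadcasting a device switch when it changes, and is re-broadcast through its own dispatcher.
; IA_Pause toggles game pause, cursor, input mode and the BP_Pause widget.
; Unpausing also re-fires the device-switch dispatcher so input prompts reflect changed mappings.
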(event `self.ReceiveBeginPlay`
  (`WidgetBlueprintLibrary.SetInputMode_GameOnly` self)
  (set `self.bShowMouseCursor` false))

(event `Key|AnyKey` :consume false :paused true :overrideparent false
  (params (Key :type "Key Structure"))
  (bind _returnvalue (`KismetInputLibrary.Key_IsGamepadKey` Key))
  (:`Pressed`
    (`|ExecutionSequence`
      (:`then_0`
        (if (!= (`self.IsUsingGamepad`) _returnvalue)
          (bind _output_get (set `self.IsUsingGamepad` _returnvalue))
          (`self.OnInputDeviceSwitched` _output_get)))
      (:`then_1`
        (`self.OnAnyKeyPressed` Key)))))

(event `EnhancedInput|/Game/Grapple/Player/Input/Actions/IA_Pause`
  (params (ActionValue :type Boolean) (ElapsedSeconds :type "Float (double-precision)") (TriggeredSeconds :type "Float (double-precision)") (InputAction :type "InputAction Object Reference" :default "/Game/Grapple/Player/Input/Actions/IA_Pause.IA_Pause"))
  (:`Started`
    (if (not (`GameplayStatics.IsGamePaused`))
      (`|ExecutionSequence`
        (:`then_0`
          (`GameplayStatics.SetGamePaused` true)
          (`WidgetBlueprintLibrary.SetInputMode_GameAndUIEx` self null)
          (set `self.bShowMouseCursor` true))
        (:`then_1`
          (bind _returnvalue (`|CreateWidget` "/Game/Grapple/Pause/BP_Pause.BP_Pause_C"))
          (bind _output_get (set `self.CurrentPauseScreen` _returnvalue))
          (`UserWidget.AddToViewport` _output_get 0)))
      (else
        (`|ExecutionSequence`
          (:`then_0`
            (`WidgetBlueprintLibrary.SetInputMode_GameOnly` self)
            (set `self.bShowMouseCursor` false))
          (:`then_1`
            (`GameplayStatics.SetGamePaused` false)
            (`Widget.RemoveFromParent` (`self.CurrentPauseScreen`)))
          (:`then_2`
            (`self.OnInputDeviceSwitched` (`self.IsUsingGamepad`)) ; is triggered once so input prompts update for changed mappings
          ))))))

(fn `UserConstructionScript`)