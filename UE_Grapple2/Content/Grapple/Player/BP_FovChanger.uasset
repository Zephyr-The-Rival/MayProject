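; BP_FovChanger is a component that widens its owning character's camera field of view with movement speed.
; On BeginPlay it caches the owner's camera component and character reference, printing a message if either is missing.
; Each Tick it maps velocity relative to MaxSpeed onto a clamped default-to-max FOV target, eases toward it with FInterpTo and applies it to the camera.
; Tick also prints the current FOV and does not validate the cached references.
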(event `self.ReceiveBeginPlay`
  (bind _returnvalue (`self.GetOwner`))
  (bind _returnvalue_2 (`Actor.GetComponentByClass` _returnvalue "/Script/Engine.CameraComponent"))
  (`/Engine/EditorBlueprintResources/StandardMacros.IsValid` _returnvalue
    (:`Is Valid`
      (`/Engine/EditorBlueprintResources/StandardMacros.IsValid` _returnvalue_2
        (:`Is Valid`
          (set `self.Camera` _returnvalue_2)
          (bind _ascharacter (cast `Character` _returnvalue)
            (:`then`
              (set `self.OwnerCharacter` _ascharacter))
            (:`CastFailed`
              (`KismetSystemLibrary.PrintString` "Owner is not a character"))))
        (:`Is Not Valid`
          (`KismetSystemLibrary.PrintString` "Owner Doesnt have a camera component"))))
    (:`Is Not Valid`
      (`KismetSystemLibrary.PrintString` "Owner is not valid"))))

(event `self.ReceiveTick`
  (params (DeltaSeconds :type "Float (single-precision)"))
  (`|ExecutionSequence`
    (:`then_0`
      (`|ExecutionSequence`
        (:`then_0`
          (set `self.Alpha` (/ (`KismetMathLibrary.VSize` (`MovementComponent.Velocity` (`Character.CharacterMovement` (`self.OwnerCharacter`)))) (`self.MaxSpeed`))))
        (:`then_1`
          (set `self.TargetFOV` (`KismetMathLibrary.FClamp` (`KismetMathLibrary.Lerp` (`self.DefaultFOV`) (`self.MaxFOV`) (`self.Alpha`)) (`self.DefaultFOV`) (`self.MaxFOV`))))
        (:`then_2`
          (bind _output_get (set `self.FOV` (`KismetMathLibrary.FInterpTo` (`self.FOV`) (`self.TargetFOV`) (`GameplayStatics.GetWorldDeltaSeconds`) (`self.FovChangeSpeed`))))
          (`KismetSystemLibrary.PrintString` (`KismetStringLibrary.Conv_DoubleToString` _output_get)))))
    (:`then_1`
      (`CameraComponent.SetFieldOfView` (`self.Camera`) (`self.FOV`)))))