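; BP_BatteryPack gives its owning grapple player character a set of batteries that recharge through movement.
; On BeginPlay it caches the owner's CharacterMovement and constructs the configured number of BP_Battery objects.
; Each Tick, while speed exceeds the charging threshold, it adds delta time to the current battery's charge, clamped to its maximum.
; Once that battery is full, charging advances to the next, stopping at the last; no discharge happens here.
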(event `self.ReceiveBeginPlay`
  (`|ExecutionSequence`
    (:`then_0`
      (bind _asbp_grapple_player_character (cast `/Game/Grapple/Player/BP_GrapplePlayerCharacter` (`self.GetOwner`)))
      (set `self.ParentCharacterMovement` (`Character.CharacterMovement` _asbp_grapple_player_character)))
    (:`then_1`
      (for _ (range (`self.NumberOfBatteries`))
        (bind _returnvalue (`|GenericCreateObject` "/Game/Grapple/Player/BatteryPack/BP_Battery.BP_Battery_C"))
        (`KismetArrayLibrary.Array_Add` (`self.Batteries`) _returnvalue)))))

(event `self.ReceiveTick`
  (params (DeltaSeconds :type "Float (single-precision)"))
  (bind _output (`|GetArrayItem` (`self.Batteries`) (`self.CurrentlyUsedBattery`)))
  (bind _output_2 (`|GetArrayItem` (`self.Batteries`) (`self.CurrentlyUsedBattery`)))
  ; ChargingBattery
  (if (> (`KismetMathLibrary.VSize` (`MovementComponent.Velocity` (`self.ParentCharacterMovement`))) (`self.ChargingThreshold`))
    (if (< (`/Game/Grapple/Player/BatteryPack/BP_Battery.Charge` _output) (`/Game/Grapple/Player/BatteryPack/BP_Battery.GetMaxCharge` _output))
      (set `/Game/Grapple/Player/BatteryPack/BP_Battery.Charge` (`KismetMathLibrary.FClamp` (+ (`/Game/Grapple/Player/BatteryPack/BP_Battery.Charge` _output_2) (`GameplayStatics.GetWorldDeltaSeconds`)) 0.0 (`/Game/Grapple/Player/BatteryPack/BP_Battery.GetMaxCharge` _output_2)) (`|GetArrayItem` (`self.Batteries`) (`self.CurrentlyUsedBattery`)))
      (elif (< (`self.CurrentlyUsedBattery`) (- (`self.NumberOfBatteries`) 1))
        (`/Engine/EditorBlueprintResources/StandardMacros.IncrementInt` (`self.CurrentlyUsedBattery`))))))