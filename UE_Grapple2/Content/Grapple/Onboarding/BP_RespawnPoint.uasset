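; Respawn point for the Grapple onboarding that moves a triggered player back to this actor behind a camera fade.
; The Triggered event starts a short camera fade, then after a matching delay places the player slightly above the point.
; It also aligns the controller's rotation to the point and zeroes movement velocity so no momentum carries over.
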(event `self.Triggered`
  (params (Player :type "/Game/Grapple/Player/BP_GrapplePlayerCharacter Object Reference"))
  (bind (_returnvalue_location _returnvalue_rotation) (`KismetMathLibrary.BreakTransform` (`self.GetTransform`)))
  ; Respawnm
  (`|ExecutionSequence`
    (:`then_0`
      (`PlayerCameraManager.StartCameraFade` :`self` (`GameplayStatics.GetPlayerCameraManager` 0) :`ToAlpha` 2.0 :`Duration` 0.5))
    (:`then_1`
      (`KismetSystemLibrary.Delay` 0.5)
      (`|ExecutionSequence`
        (:`then_0`
          (`self.K2_SetActorLocation` Player (+ _returnvalue_location (0.0 0.0 200.0)) false false)
          (`Controller.SetControlRotation` (`Pawn.GetController` Player) _returnvalue_rotation))
        (:`then_1`
          (set `MovementComponent.Velocity` (0.0 0.0 0.0) (`Character.CharacterMovement` Player)))))))

(fn `UserConstructionScript`)