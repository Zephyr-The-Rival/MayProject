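; Grapple onboarding launcher that flings the player along its Arrow's forward vector when they overlap either detector.
; Deterministic mode uses a timeline to lerp the player to the arrow, then sets their velocity to a fixed strength.
; Dynamic mode adds a velocity-change impulse but never clears the Launching guard, so it fires only once.
; In deterministic mode, the construction script draws an approximate arc preview spline, which is destroyed on BeginPlay.
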(event `self.ReceiveBeginPlay`
  (bind _debugspline (`self.DebugSpline`))
  (`/Engine/EditorBlueprintResources/StandardMacros.IsValid` _debugspline
    (:`Is Valid`
      (`ActorComponent.K2_DestroyComponent` _debugspline))))

(event `self.Playerdetector1.OnComponentBeginOverlap`
  (params (OverlappedComponent :type "PrimitiveComponent Object Reference") (OtherActor :type "Actor Object Reference") (OtherComp :type "PrimitiveComponent Object Reference") (OtherBodyIndex :type Integer) (bFromSweep :type Boolean) (SweepResult :type "HitResult Structure (by ref)"))
  (bind _asbp_grapple_player_character (cast `/Game/Grapple/Player/BP_GrapplePlayerCharacter` OtherActor))
  (`self.LaunchPlayer` _asbp_grapple_player_character))

(event `self.Playerdetector.OnComponentBeginOverlap`
  (params (OverlappedComponent :type "PrimitiveComponent Object Reference") (OtherActor :type "Actor Object Reference") (OtherComp :type "PrimitiveComponent Object Reference") (OtherBodyIndex :type Integer) (bFromSweep :type Boolean) (SweepResult :type "HitResult Structure (by ref)"))
  (bind _asbp_grapple_player_character (cast `/Game/Grapple/Player/BP_GrapplePlayerCharacter` OtherActor))
  (`self.LaunchPlayer` _asbp_grapple_player_character))

(event `LaunchPlayer`
  (params (Player :type "/Game/Grapple/Player/BP_GrapplePlayerCharacter Object Reference"))
  (bind _playertolaunch (`self.PlayerToLaunch`))
  (if (not (`self.Launching`))
    (set `self.Launching` true)
    (set `self.PlayerToLaunch` Player)
    (if (`self.DeterministicLaunch`)
      (`|ExecutionSequence`
        (:`then_0`
          (set `self.PlayerStartLoaction` (`self.K2_GetActorLocation` _playertolaunch))
          (set `self.PlayerStartVelocity` (`CharacterMovementComponent.GetLastUpdateRequestedVelocity` (`Character.CharacterMovement` _playertolaunch))))
        (:`then_1`
          (bind (_direction _0_to_1) (`Timeline|ChangePlayerPosition & Velocity` :!via `PlayFromStart`)
            (:`Update`
              (`|ExecutionSequence`
                (:`then_0`
                  (`self.K2_SetActorLocation` (`self.PlayerToLaunch`) (`KismetMathLibrary.VLerp` (`self.PlayerStartLoaction`) (`SceneComponent.K2_GetComponentLocation` (`self.Arrow`)) _0_to_1) false false))))
            (:`Finished`
              (set `MovementComponent.Velocity` (* (`SceneComponent.GetForwardVector` (`self.Arrow`)) (`self.DeterministicLaunchStrenght`)) (`Character.CharacterMovement` (`self.PlayerToLaunch`)))
              (set `self.Launching` false)))))
      (else
        (`CharacterMovementComponent.AddImpulse` (`Character.CharacterMovement` (`self.PlayerToLaunch`)) (* (`SceneComponent.GetForwardVector` (`self.Arrow`)) (`self.DynamicLaunchStrenght`)) true)))))

(fn `UserConstructionScript`
  (locals (Points :type "Array of Vector Structure"))
  (bind _debugspline (`self.DebugSpline`))
  (if (`self.DeterministicLaunch`)
    (`|ExecutionSequence`
      (:`then_0`
        (for _index (range 51)
          (bind _returnvalue (* (`KismetMathLibrary.Conv_IntToDouble` _index) 0.1))
          (`KismetArrayLibrary.Array_Add` (`local.Points`) (+ (`SceneComponent.K2_GetComponentLocation` (`self.Arrow`)) (* (* (`SceneComponent.GetForwardVector` (`self.Arrow`)) (* (`self.DeterministicLaunchStrenght`) 1.4)) _returnvalue) (* (0.0 0.0 -1.0) (0.0 0.0 981.0) (`KismetMathLibrary.MultiplyMultiply_FloatFloat` _returnvalue 2.0))))))
      (:`then_1`
        (`|ExecutionSequence`
          (:`then_0`
            (`/Engine/EditorBlueprintResources/StandardMacros.IsValid` _debugspline
              (:`Is Valid`
                (`ActorComponent.K2_DestroyComponent` _debugspline))))
          (:`then_1`
            (bind _returnvalue_2 (`AddComponent|NODE_AddSplineComponent-1` :`RelativeTransform` (`KismetMathLibrary.MakeTransform` (`SceneComponent.RelativeLocation` (`self.Arrow`)))))
            (set `self.DebugSpline` _returnvalue_2))
          (:`then_2`
            (for (_array_element _array_index) (`local.Points`)
              (if (!= _array_index 0)
                (`SplineComponent.AddSplinePoint` (`self.DebugSpline`) _array_element "World" true)))))))))