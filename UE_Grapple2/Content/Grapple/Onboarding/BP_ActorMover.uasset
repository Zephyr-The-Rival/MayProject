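; BP_ActorMover is a triggerable Blueprint that moves a referenced actor between two locations, either on BeginPlay or when triggered.
; Tick linearly interpolates the actor's location over Duration without sweeping, then snaps it to the end point.
; With Loop enabled it swaps start and end and restarts, producing a ping-pong motion.
; The construction script can auto-capture the start location from the actor's placed position.
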(event `self.ReceiveBeginPlay`
  (if (`self.PlayFromStart`)
    (`self.StartMove`)))

(event `self.Triggered`
  (params (Player :type "/Game/Grapple/Player/BP_GrapplePlayerCharacter Object Reference"))
  (`parent.Triggered` Player)
  (`self.StartMove`))

(event `StartMove`
  (`/Engine/EditorBlueprintResources/StandardMacros.IsValid` (`self.ActorToMove`)
    (:`Is Valid`
      (set `self.Time Counter` 0.0)
      (set `self.Move` true))
    (:`Is Not Valid`
      (`KismetSystemLibrary.PrintString` "ActorToMove Is not valid"))))

(event `self.ReceiveTick`
  (params (DeltaSeconds :type "Float (single-precision)"))
  (bind _returnvalue (/ (`self.Time Counter`) (`self.Duration`)))
  (if (`self.Move`)
    (`|ExecutionSequence`
      (:`then_0`
        (set `self.Time Counter` (+ (`self.Time Counter`) (`GameplayStatics.GetWorldDeltaSeconds`))))
      (:`then_1`
        (if (>= _returnvalue 1.0)
          (`self.K2_SetActorLocation` (`self.ActorToMove`) (`self.EndLocation`) false false)
          (set `self.Move` false)
          (if (`self.Loop`)
            (`|ExecutionSequence`
              (:`then_0`
                (set `self.EndLocation` (`self.StartLocation`))
                (set `self.StartLocation` (`self.K2_GetActorLocation` (`self.ActorToMove`))))
              (:`then_1`
                (`self.StartMove`))))
          (else
            (`self.K2_SetActorLocation` (`self.ActorToMove`) (`KismetMathLibrary.VLerp` (`self.StartLocation`) (`self.EndLocation`) _returnvalue) false false)))))))

(fn `UserConstructionScript`
  (if (and (`KismetSystemLibrary.IsValid` (`self.ActorToMove`)) (`self.AutoSetStartPos`))
    (set `self.StartLocation` (`self.K2_GetActorLocation` (`self.ActorToMove`)))))