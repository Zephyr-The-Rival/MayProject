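; BP_BoosterField is a boost volume that pushes the grapple player character along the field's forward vector.
; When its box begins overlapping that character, it calls Boost, which checks the player's slide and wallrun components.
; Ground sliding triggers AddBoost on BP_Slide and wallrunning triggers ApplyBoost on BP_WallRun, each scaled by its own strength.
; The boost fires only on overlap begin and does nothing in other movement states.
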(event `self.Box.OnComponentBeginOverlap`
  (params (OverlappedComponent :type "PrimitiveComponent Object Reference") (OtherActor :type "Actor Object Reference") (OtherComp :type "PrimitiveComponent Object Reference") (OtherBodyIndex :type Integer) (bFromSweep :type Boolean) (SweepResult :type "HitResult Structure (by ref)"))
  (bind _asbp_grapple_player_character (cast `/Game/Grapple/Player/BP_GrapplePlayerCharacter` OtherActor))
  (`self.Boost` _asbp_grapple_player_character))

(event `Boost`
  (params (Player :type "/Game/Grapple/Player/BP_GrapplePlayerCharacter Object Reference"))
  (bind _slider (`GrapplePlayerCharacter.Slider` Player))
  (bind _wallrunner (`GrapplePlayerCharacter.Wallrunner` Player))
  (`|ExecutionSequence`
    (:`then_0`
      (if (`Slide.bSlidingOnGround` _slider)
        (bind _asbp_slide (cast `/Game/Grapple/Player/BP_Slide` _slider))
        (`/Game/Grapple/Player/BP_Slide.AddBoost` _asbp_slide (* (`self.GetActorForwardVector`) (`self.BoostStrenghtSlide`)))))
    (:`then_1`
      (if (`Wallrun.bWallrunning` _wallrunner)
        (bind _asbp_wall_run (cast `/Game/Grapple/Player/BP_WallRun` _wallrunner))
        (`/Game/Grapple/Player/BP_WallRun.ApplyBoost` _asbp_wall_run (* (`self.GetActorForwardVector`) (`self.BoostStrenghtWallrun`)))))))

(fn `UserConstructionScript`)