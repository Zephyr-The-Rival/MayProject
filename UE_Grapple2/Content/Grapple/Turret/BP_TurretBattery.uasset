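; BP_TurretBattery is a turret's battery that the player can grapple to and kick.
; Grapples target the static mesh's center of mass.
; Each tick, Sphere collision switches to query-only while the player camera's forward roughly matches KickDirectionArrow, otherwise it is disabled.
; Kicks above a minimum strength defer to the parent implementation; weaker ones print a message and return a dampened, reversed kick vector.
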(event `self.ReceiveTick`
  (params (DeltaSeconds :type "Float (single-precision)"))
  (bind _sphere (`self.Sphere`))
  (`parent.ReceiveTick` DeltaSeconds)
  (bind _asbp_grapple_player_character (cast `/Game/Grapple/Player/BP_GrapplePlayerCharacter` (`GameplayStatics.GetPlayerPawn` 0)))
  (if (> (`KismetMathLibrary.Dot_VectorVector` (`SceneComponent.GetForwardVector` (`GrapplePlayerCharacter.Camera` _asbp_grapple_player_character)) (`SceneComponent.GetForwardVector` (`self.KickDirectionArrow`))) 0.5)
    (`PrimitiveComponent.SetCollisionEnabled` _sphere "QueryOnly")
    (else
      (`PrimitiveComponent.SetCollisionEnabled` _sphere "NoCollision"))))

(fn `GetGrappleLocation`
  (returns (GrappleLocation :type "Vector Structure"))
  (return (`PrimitiveComponent.GetCenterOfMass` (`self.StaticMesh`) "None")))

(fn `Kick`
  (params (TheKicker :type "/Game/Grapple/Player/BP_GrapplePlayerCharacter Object Reference") (Direction :type "Vector Structure") (Strenght :type "Float (double-precision)"))
  (returns (PostKickPlayerVelocity :type "Vector Structure"))
  (if (> Strenght (`self.Min Kick Strenght`))
    (bind _postkickplayervelocity (`parent.Kick` TheKicker Direction Strenght))
    (return _postkickplayervelocity)
    (else
      (`KismetSystemLibrary.PrintString` "NOT ENOUGH KICK SPEED")
      (return (* Direction (* Strenght -0.7))))))

(fn `UserConstructionScript`
  (`parent.UserConstructionScript`))