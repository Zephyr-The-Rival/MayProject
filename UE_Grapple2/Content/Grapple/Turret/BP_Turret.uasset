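; Turret actor that tracks the player pawn and fires bullets, with a child-actor battery as its weak point.
; While active, Tick yaws the head and pitches the clamped barrels toward the player at constant speed.
; When roughly aimed, a Delay throttles bullet spawns from every barrel socket.
; Battery events swap turn speed while hooked, restore it on release, and destroy the turret with a Niagara effect when kicked.
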(event `self.ReceiveBeginPlay`
  (bind _asbp_turret_battery (cast `/Game/Grapple/Turret/BP_TurretBattery` (`ChildActorComponent.ChildActor` (`self.BP_TurretBattery`))))
  (add `/Game/Grapple/GrappleObjects/BP_Kick_GrappleObject.OnLetGo` _asbp_turret_battery (`|CreateDelegate` :!event `OnBatteryLetGo`))
  (add `/Game/Grapple/GrappleObjects/BP_Kick_GrappleObject.OnHooked` _asbp_turret_battery (`|CreateDelegate` :!event `OnBatteryHooked`))
  (add `/Game/Grapple/GrappleObjects/BP_Kick_GrappleObject.OnKicked` _asbp_turret_battery (`|CreateDelegate` :!event `OnKicked`)))

(event `self.ReceiveTick`
  (params (DeltaSeconds :type "Float (single-precision)"))
  (bind _returnvalue (`GameplayStatics.GetPlayerPawn` 0))
  (bind _returnvalue_2 (`GameplayStatics.GetPlayerPawn` 0))
  (bind _barrels (`self.Barrels`))
  ; TurnHead
  (if (`self.Active`)
    (`|ExecutionSequence`
      (:`then_0`
        (`/Engine/EditorBlueprintResources/StandardMacros.IsValid` _returnvalue
          (:`Is Valid`
            (`SceneComponent.K2_SetWorldRotation` (`self.Top`) (`KismetMathLibrary.RInterpTo_Constant` (`SceneComponent.K2_GetComponentRotation` (`self.Top`)) (`KismetMathLibrary.Conv_VectorToRotator` (* (- (`self.K2_GetActorLocation` _returnvalue) (`SceneComponent.K2_GetComponentLocation` (`self.Top`))) (1.0 1.0 0.0))) (`GameplayStatics.GetWorldDeltaSeconds`) (`self.TurnSpeed`)) false false))))
      (:`then_1`
        ; Turn Barrels
        (`/Engine/EditorBlueprintResources/StandardMacros.IsValid` _returnvalue_2
          (:`Is Valid`
            (`SceneComponent.K2_SetRelativeRotation` (`self.Barrels`) (`KismetMathLibrary.MakeRotator` 0.0 (`KismetMathLibrary.ClampAngle` (.pitch (`KismetMathLibrary.RInterpTo_Constant` (`SceneComponent.RelativeRotation` (`self.Barrels`)) (`KismetMathLibrary.MakeRotFromX` (- (.location (`KismetMathLibrary.MakeRelativeTransform` (`self.GetTransform` _returnvalue_2) (`SceneComponent.K2_GetComponentToWorld` (`self.Top`)))) (`SceneComponent.RelativeLocation` (`self.Barrels`)))) (`GameplayStatics.GetWorldDeltaSeconds`) (`self.TurnSpeed`))) -25.0 25.0)) false false))))
      (:`then_2`
        ; SpawnBuleltrs
        (if (> (`KismetMathLibrary.Dot_VectorVector` (`KismetMathLibrary.Normal` (- (`self.K2_GetActorLocation` (`GameplayStatics.GetPlayerPawn` 0)) (`SceneComponent.K2_GetComponentLocation` _barrels))) (`SceneComponent.GetForwardVector` _barrels)) 0.8)
          (`KismetSystemLibrary.Delay` 0.7)
          (`self.Spawn Bullet`))))))

(event `Spawn Bullet`
  (bind _barrels (`self.Barrels`))
  ; SpawnBuleltrs
  (for _array_element (`SceneComponent.GetAllSocketNames` _barrels)
    (`|SpawnActorFromClass` "/Game/Grapple/Turret/BP_Bullet.BP_Bullet_C" (`SceneComponent.GetSocketTransform` _barrels _array_element "RTS_World") "Undefined" "MultiplyWithRoot" null null)))

(event `OnKicked`
  (params (Kicker :type "/Game/Grapple/Player/BP_GrapplePlayerCharacter Object Reference") (Direction :type "Vector Structure") (Strenght :type "Float (double-precision)"))
  (`NiagaraFunctionLibrary.SpawnSystemAttached` "/Game/Effects/ImpactEffects/NS_Wobble.NS_Wobble" null "None" (0.0 0.0 0.0) (struct) "KeepRelativeOffset")
  (`self.K2_DestroyActor`))

(event `OnBatteryHooked`
  (set `self.TurnSpeed` (`self.HookedTurnSpeed`)))

(event `OnBatteryLetGo`
  (set `self.TurnSpeed` (defaults `/Game/Grapple/Turret/BP_Turret` "BP_Turret_C")))

(fn `UserConstructionScript`)