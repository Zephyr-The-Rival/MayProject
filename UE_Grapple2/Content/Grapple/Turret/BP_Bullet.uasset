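; BP_Bullet is a turret projectile in the Grapple game that flies straight and detects hits on the player.
; Each tick it moves along its forward vector at MovementSpeed with a swept world offset, so the sweep itself provides collision detection.
; A blocking hit destroys it, printing a debug message if the hit actor is BP_GrapplePlayerCharacter; no damage is applied.
; It also destroys itself after a fixed lifetime delay.
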(event `self.ReceiveBeginPlay`
  (`KismetSystemLibrary.Delay` 30.0)
  (`self.K2_DestroyActor`))

(event `self.ReceiveTick`
  (params (DeltaSeconds :type "Float (single-precision)"))
  (bind _sweephitresult (`self.K2_AddActorWorldOffset` (* (`self.GetActorForwardVector`) (`self.MovementSpeed`) (`GameplayStatics.GetWorldDeltaSeconds`)) true))
  (bind (_bblockinghit _binitialoverlap _time _distance _location _impactpoint _normal _impactnormal _physmat _hitactor) (`GameplayStatics.BreakHitResult` _sweephitresult))
  (if _bblockinghit
    (`|ExecutionSequence`
      (:`then_0`
        (cast `/Game/Grapple/Player/BP_GrapplePlayerCharacter` _hitactor)
        (`KismetSystemLibrary.PrintString` "Bullet hit player"))
      (:`then_1`
        (`self.K2_DestroyActor`)))))

(fn `UserConstructionScript`)