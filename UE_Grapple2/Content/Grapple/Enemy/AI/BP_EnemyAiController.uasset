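; AI controller for enemies in the Grapple game, which starts the BT_Enemy behavior tree when it possesses a pawn.
; Each tick, while the player pawn is valid, it line traces on the Visibility channel from the controlled pawn to the player.
; It writes the inverted hit result to the HasLineOfSight blackboard key, so an unblocked trace counts as seeing the player.
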(event `self.ReceivePossess`
  (params (PossessedPawn :type "Pawn Object Reference"))
  (`self.RunBehaviorTree` "/Game/Grapple/Enemy/AI/BT_Enemy.BT_Enemy"))

(event `self.ReceiveTick`
  (params (DeltaSeconds :type "Float (single-precision)"))
  (bind _returnvalue (`GameplayStatics.GetPlayerPawn` 0))
  (`/Engine/EditorBlueprintResources/StandardMacros.IsValid` _returnvalue
    (:`Is Valid`
      (bind (_outhit _returnvalue_2) (`KismetSystemLibrary.LineTraceSingle` (`self.K2_GetActorLocation` (`self.K2_GetPawn`)) (`self.K2_GetActorLocation` _returnvalue) "TraceTypeQuery1"))
      (`BlackboardComponent.SetValueAsBool` (`AIBlueprintHelperLibrary.GetBlackboard` null) "HasLineOfSight" (not _returnvalue_2)))))

(fn `UserConstructionScript`)