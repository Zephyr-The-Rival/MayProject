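; Enemy gun actor that fires BP_EnemyBullet projectiles automatically while its trigger is held.
; Pull and release events set a flag that Tick polls to call Fire, which spawns a bullet at the skeletal mesh's Muzzle socket.
; Each shot starts a FireRate cooldown timer that blocks refiring, then calls OnFired.
; Releasing the trigger pauses that timer, so the next pull can fire immediately.
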(event `PullTrigger`
  (set `self.TriggerPulled` true))

(event `self.ReceiveTick`
  (params (DeltaSeconds :type "Float (single-precision)"))
  (if (`self.TriggerPulled`)
    (`self.Fire`)))

(event `ReleaseTrigger`
  (set `self.TriggerPulled` false)
  (`KismetSystemLibrary.K2_PauseTimerHandle` (`self.FireCooldownTimer`)))

(event `Fire`
  (if (not (`KismetSystemLibrary.K2_IsTimerActiveHandle` (`self.FireCooldownTimer`)))
    (`|ExecutionSequence`
      (:`then_0`
        (`|SpawnActorFromClass` "/Game/Grapple/Enemy/BP_EnemyBullet.BP_EnemyBullet_C" (`SceneComponent.GetSocketTransform` (`self.SkeletalMesh`) "Muzzle" "RTS_World") "Undefined" "MultiplyWithRoot" null null))
      (:`then_1`
        (bind _returnvalue (`KismetSystemLibrary.K2_SetTimerDelegate` (`|CreateDelegate` :!event `Fire`) (`self.FireRate`)))
        (set `self.FireCooldownTimer` _returnvalue))
      (:`then_2`
        (`self.OnFired`)))))

(fn `UserConstructionScript`)