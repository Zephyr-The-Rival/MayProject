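; Grapple kick object for enemies, serving as the point the player grapples to and kicks off from.
; It expects BP_Enemy as its parent actor and overrides the grapple location to that enemy's mesh spine_03 socket.
; The post-kick player velocity reverses the incoming direction at a fixed bounce-back strength, discarding the original speed.
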(fn `CalculatePostKickPlayerVelocity`
  (params (OldVelocity :type "Vector Structure"))
  (returns (NewVelocity :type "Vector Structure"))
  (return (* (`KismetMathLibrary.NegateVector` (`KismetMathLibrary.Normal` OldVelocity)) (`self.KickBouncebackStrenght`))))

(fn `GetGrappleLocation`
  (returns (GrappleLocation :type "Vector Structure"))
  (bind _asbp_enemy (cast `/Game/Grapple/Enemy/BP_Enemy` (`self.GetParentActor`)))
  (return (`SceneComponent.GetSocketLocation` (`Character.Mesh` _asbp_enemy) "spine_03")))

(fn `UserConstructionScript`
  (`parent.UserConstructionScript`))