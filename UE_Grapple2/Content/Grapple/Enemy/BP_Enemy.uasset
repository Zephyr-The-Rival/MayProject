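; BP_Enemy is an armed, AI-controlled enemy that reacts to being grappled and kicked.
; On BeginPlay it attaches a spawned gun, binds to its fired event for recoil animation, and tints the mesh materials with a team color.
; A child-actor grapple/kick object reports hits: hooking stops the behavior logic and firing, while a kick plays a random death montage that clears the hooked flag on completion.
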(event `self.ReceiveBeginPlay`
  (bind _mesh (`self.Mesh`))
  (`|ExecutionSequence`
    (:`then_0`
      (bind _returnvalue (`|SpawnActorFromClass` "/Game/Grapple/Enemy/BP_EnemyGun.BP_EnemyGun_C" (`KismetMathLibrary.MakeTransform` (0.0 0.0 0.0)) "Undefined" "MultiplyWithRoot" null null))
      (set `self.MyGun` _returnvalue)
      (`self.K2_AttachToComponent` _returnvalue (`self.Mesh`) "weapon_r" "SnapToTarget" "SnapToTarget" "SnapToTarget" true)
      (add `/Game/Grapple/Enemy/BP_EnemyGun.OnFired` (`self.MyGun`) (`|CreateDelegate` :!event `GunfireRecoil`)))
    (:`then_1`
      (bind _asbp_enemy_grapple_kick_object (cast `/Game/Grapple/Enemy/BP_EnemyGrappleKickObject` (`ChildActorComponent.ChildActor` (`self.EnemyGrappleObject`))))
      (add `/Game/Grapple/GrappleObjects/BP_Kick_GrappleObject.OnHooked` _asbp_enemy_grapple_kick_object (`|CreateDelegate` :!event `GrappleHooked`))
      (add `/Game/Grapple/GrappleObjects/BP_Kick_GrappleObject.OnKicked` _asbp_enemy_grapple_kick_object (`|CreateDelegate` :!event `OnKicked`)))
    (:`then_2`
      (for (_array_element _array_index) (`MeshComponent.GetMaterials` _mesh)
        (bind _returnvalue_2 (`PrimitiveComponent.CreateDynamicMaterialInstance` _mesh _array_index _array_element "None"))
        (`MaterialInstanceDynamic.SetVectorParameterValue` _returnvalue_2 "TeamColor" (struct :`R` 0.097049 :`G` 0.829794 :`B` 1.0 :`A` 1.0))))))

(event `SetTriggerPulled`
  (params (NewPulled :type Boolean))
  (bind _mygun (`self.MyGun`))
  ; PullTrigger
  (if NewPulled
    (`/Game/Grapple/Enemy/BP_EnemyGun.PullTrigger` _mygun)
    (else
      (`/Game/Grapple/Enemy/BP_EnemyGun.ReleaseTrigger` _mygun))))

(event `self.ReceiveTick`
  (params (DeltaSeconds :type "Float (single-precision)")))

(event `GunfireRecoil`
  (`|PlayMontage` (`self.Mesh`) "/Game/Characters/Heroes/Mannequin/Animations/Actions/MM_Rifle_Fire_Montage.MM_Rifle_Fire_Montage"))

(event `GrappleHooked`
  (bind _returnvalue (`AIBlueprintHelperLibrary.GetAIController` self))
  (`/Engine/EditorBlueprintResources/StandardMacros.IsValid` _returnvalue
    (:`Is Valid`
      (`|ExecutionSequence`
        (:`then_0`
          (`BrainComponent.StopLogic` (`AIController.BrainComponent` _returnvalue) "Hooked"))
        (:`then_1`
          (`self.SetTriggerPulled` false))
        (:`then_2`
          (set `self.Hooked` true))))))

(event `OnKicked`
  (params (Kicker :type "/Game/Grapple/Player/BP_GrapplePlayerCharacter Object Reference") (Direction :type "Vector Structure") (Strenght :type "Float (double-precision)"))
  (`|PlayMontage` (`self.Mesh`) (`KismetArrayLibrary.Array_Random` (`|MakeArray` "/Game/Characters/Heroes/Mannequin/Animations/Actions/MM_Death_Front_01_Montage.MM_Death_Front_01_Montage" "/Game/Characters/Heroes/Mannequin/Animations/Actions/MM_Death_Front_02_Montage.MM_Death_Front_02_Montage" "/Game/Characters/Heroes/Mannequin/Animations/Actions/MM_Death_Front_03_Montage.MM_Death_Front_03_Montage" :!type "AnimMontage Object Reference"))
    (:`OnCompleted`
      (set `self.Hooked` false))))

(fn `UserConstructionScript`)