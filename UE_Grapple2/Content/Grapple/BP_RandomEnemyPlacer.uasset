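; BP_RandomEnemyPlacer is meant to scatter BP_Enemy pawns at random spots, but its spawn loop is unwired and BeginPlay does nothing.
; The loop would use ForLoopOverTime to spawn enemies up to EnemiesAmount, each possessed by a new BP_EnemyAiController.
; GetRandomLocation traces down from a random point SpawnArea away from world origin, returning the hit or zero on a miss.
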(event `self.ReceiveBeginPlay`)

(fn `GetRandomLocation`
  (returns (Location :type "Vector Structure"))
  (locals (Point :type "Vector Structure"))
  (bind _point (`local.Point`))
  (set `local.Point` (* (`KismetMathLibrary.RandomUnitVector`) (`self.SpawnArea`)))
  (bind (_outhit _returnvalue) (`KismetSystemLibrary.LineTraceSingle` :`Start` _point :`End` (- _point (`KismetMathLibrary.MakeVector` 0.0 0.0 (`self.SpawnArea`))) :`TraceChannel` "TraceTypeQuery1" :`DrawDebugType` "ForDuration"))
  (if _returnvalue
    (return (`.Location` (`GameplayStatics.BreakHitResult` _outhit)))
    (else
      (return (0.0 0.0 0.0)))))

(fn `UserConstructionScript`)