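; Blueprint function library for input prompts that resolves the icon texture and bound key for an Enhanced Input action.
; GetPromptTexture returns a gamepad or mouse-and-keyboard override if given, otherwise asks the BP_PromptTextureSupplier actor found in the level.
; Distinct placeholder textures flag a missing action, mapping context, supplier or texture.
; GetMappedKeyOfAction scans the mapping context's default mappings for the action's first key of the requested device type.
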(fn `GetMappedKeyOfAction`
  (params (Action :type "Object Object Reference") (MappingContext :type "InputMappingContext Object Reference") (LookingForGamepadKey :type Boolean))
  (returns (Key :type "Key Structure"))
  (for _array_element (`.Mappings` (break `InputMappingContextMappingData` (`InputMappingContext.DefaultKeyMappings` MappingContext)))
    (bind (_triggers _modifiers _action _key) (break `EnhancedActionKeyMapping` _array_element))
    (if (and (== (`KismetInputLibrary.Key_IsGamepadKey` _key) LookingForGamepadKey) (== Action _action))
      (return _key)))
  (return "None"))

(fn `GetPromptTexture`
  (params (Action :type "InputAction Object Reference") (MappingContext :type "InputMappingContext Object Reference") (OverrideGamepadTexture :type "Texture2D Object Reference") (OverrideMaKTexture :type "Texture2D Object Reference") (Gamepad :type Boolean))
  (returns (Texture :type "Texture2D Object Reference"))
  (`|ExecutionSequence`
    (:`then_0`
      (if (not (`KismetSystemLibrary.IsValid` (`local.Action`)))
        (return "/Game/InputPrompts/Textures/Errors/T_NoActionSelected.T_NoActionSelected")))
    (:`then_1`
      (if (not (`KismetSystemLibrary.IsValid` (`local.MappingContext`)))
        (return "/Game/InputPrompts/Textures/Errors/T_NoMappingContextSelected.T_NoMappingContextSelected")))
    (:`then_3`
      (bind _returnvalue (`GameplayStatics.GetActorOfClass` (`local.__WorldContext`) "/Game/InputPrompts/BP_PromptTextureSupplier.BP_PromptTextureSupplier_C"))
      (`/Engine/EditorBlueprintResources/StandardMacros.IsValid` _returnvalue
        (:`Is Valid`
          (`|ExecutionSequence`
            (:`then_0`
              ;[1 1 1] OverrideTextures
              (`|ExecutionSequence`
                (:`then_0`
                  (if (and (`KismetSystemLibrary.IsValid` (`local.OverrideGamepadTexture`)) (`local.Gamepad`))
                    (return (`local.OverrideGamepadTexture`))))
                (:`then_1`
                  (if (and (`KismetSystemLibrary.IsValid` (`local.OverrideMaKTexture`)) (not (`local.Gamepad`)))
                    (return (`local.OverrideMaKTexture`))))))
            (:`then_1`
              (bind _returnvalue_2 (`/Game/InputPrompts/BP_PromptTextureSupplier.GetActionTexture` _returnvalue (`local.Action`) (`local.MappingContext`) (`local.Gamepad`))) ; Get texture from supplier
              (`/Engine/EditorBlueprintResources/StandardMacros.IsValid` _returnvalue_2
                (:`Is Valid`
                  (return _returnvalue_2))
                (:`Is Not Valid`
                  (return "/Game/InputPrompts/Textures/Errors/T_NoTextureAviable.T_NoTextureAviable"))))))
        (:`Is Not Valid`
          (return "/Game/InputPrompts/Textures/Errors/T_NoTextureSupplierFound.T_NoTextureSupplierFound"))))))