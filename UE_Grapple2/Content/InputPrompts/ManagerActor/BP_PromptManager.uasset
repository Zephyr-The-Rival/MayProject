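; Input prompt manager actor that looks up which key is bound to an input action.
; On BeginPlay it has the user mappings save manager apply saved user mappings to the PlayerCharacterInput mapping context.
; GetKeyFromAction scans a given context's default key mappings and returns the first key matching both the action and the requested device type, gamepad or non-gamepad.
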(event `self.ReceiveBeginPlay`
  (`/Game/InputPrompts/ManagerActor/BP_UserMappingsSaveManager.ApplyUserSavedMappignsForMappingContext` (`self.BP_UserMappingsSaveManager`) "/Game/Grapple/Player/Input/PlayerCharacterInput.PlayerCharacterInput"))

(fn `GetKeyFromAction`
  (params (Action :type "Object Object Reference") (MappingContext :type "InputMappingContext Object Reference") (LookingForGamepadKey :type Boolean))
  (returns (Key :type "Key Structure"))
  (for _array_element (`.Mappings` (break `InputMappingContextMappingData` (`InputMappingContext.DefaultKeyMappings` MappingContext)))
    (bind (_triggers _modifiers _action _key) (break `EnhancedActionKeyMapping` _array_element))
    (if (and (== (`KismetInputLibrary.Key_IsGamepadKey` _key) LookingForGamepadKey) (== Action _action))
      (return _key))))

(fn `UserConstructionScript`)