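; Manager that persists player key rebinds for Enhanced Input mapping contexts in a BP_ControlSave save slot.
; Applying loads or creates the save, caches it, then unmaps and remaps matching actions in the given context's default mappings.
; Saving replaces the matching entry in that cached object and writes the slot.
; Both match on action and gamepad versus non-gamepad key, so a controller rebind never overwrites a keyboard one.
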(fn `ApplyUserSavedMappignsForMappingContext`
  (params (MappingContext :type "InputMappingContext Object Reference"))
  (locals (CurrentUserMappingToApply :type "/Game/InputPrompts/ManagerActor/Saving/SavedMapping Structure") (CurrentMappingToOverride :type "EnhancedActionKeyMapping Structure"))
  (bind _currentusermappingtoapply_mappingcontext (break `/Game/InputPrompts/ManagerActor/Saving/SavedMapping` (`local.CurrentUserMappingToApply`)))
  (bind _currentusermappingtoapply_mappingcontext_2 (break `/Game/InputPrompts/ManagerActor/Saving/SavedMapping` (`local.CurrentUserMappingToApply`)))
  (bind (_currentusermappingtoapply_mappingcontext_3 _currentusermappingtoapply_action _currentusermappingtoapply_mappedkey) (break `/Game/InputPrompts/ManagerActor/Saving/SavedMapping` (`local.CurrentUserMappingToApply`)))
  (bind (_currentmappingtooverride_triggers _currentmappingtooverride_modifiers _currentmappingtooverride_action _currentmappingtooverride_key) (break `EnhancedActionKeyMapping` (`local.CurrentMappingToOverride`)))
  (bind (_currentmappingtooverride_triggers_2 _currentmappingtooverride_modifiers_2 _currentmappingtooverride_action_2 _currentmappingtooverride_key_2) (break `EnhancedActionKeyMapping` (`local.CurrentMappingToOverride`)))
  (bind (_currentusermappingtoapply_mappingcontext_4 _currentusermappingtoapply_action_2 _currentusermappingtoapply_mappedkey_2) (break `/Game/InputPrompts/ManagerActor/Saving/SavedMapping` (`local.CurrentUserMappingToApply`)))
  (`|ExecutionSequence`
    (:`then_0`
      (bind _usedmappingsave (`self.LoadMappingsSave`))
      (set `self.SavedControls` _usedmappingsave))
    (:`then_1`
      (if (`/Game/InputPrompts/ManagerActor/Saving/BP_ControlSave.ContainsAlteredMappings` (`self.SavedControls`))
        (for _array_element (`/Game/InputPrompts/ManagerActor/Saving/BP_ControlSave.SavedMappings` (`self.SavedControls`))
          (set `local.CurrentUserMappingToApply` _array_element)
          (`/Engine/EditorBlueprintResources/StandardMacros.IsValid` _currentusermappingtoapply_mappingcontext
            (:`Is Valid`
              (if (== _currentusermappingtoapply_mappingcontext_2 (`local.MappingContext`))
                (for _array_element_2 (`.Mappings` (break `InputMappingContextMappingData` (`InputMappingContext.DefaultKeyMappings` (`local.MappingContext`))))
                  (set `local.CurrentMappingToOverride` _array_element_2)
                  (if (and (== _currentmappingtooverride_action _currentusermappingtoapply_action) (== (`KismetInputLibrary.Key_IsGamepadKey` _currentmappingtooverride_key) (`KismetInputLibrary.Key_IsGamepadKey` _currentusermappingtoapply_mappedkey)))
                    (`|ExecutionSequence`
                      (:`then_0`
                        (`InputMappingContext.UnmapKey` (`local.MappingContext`) _currentmappingtooverride_action_2 _currentmappingtooverride_key_2) ; unmapping old key
                      )
                      (:`then_1`
                        (`InputMappingContext.MapKey` (`local.MappingContext`) _currentusermappingtoapply_action_2 _currentusermappingtoapply_mappedkey_2) ; mapping new key
                      ))))))
            (:`Is Not Valid`
              (`KismetSystemLibrary.PrintString` "Saved Mapping context object reference is not valid"))))
        (else
          (return))))))

(fn `LoadMappingsSave`
  (returns (UsedMappingSave :type "/Game/InputPrompts/ManagerActor/Saving/BP_ControlSave Object Reference"))
  (bind _returnvalue (`GameplayStatics.DoesSaveGameExist` (`self.SaveName`)))
  (if _returnvalue
    (bind _returnvalue_2 (`GameplayStatics.LoadGameFromSlot` (`self.SaveName`)))
    (bind _asbp_control_save (cast `/Game/InputPrompts/ManagerActor/Saving/BP_ControlSave` _returnvalue_2))
    (return _asbp_control_save)
    (else
      (bind _returnvalue_3 (`GameplayStatics.CreateSaveGameObject` "/Game/InputPrompts/ManagerActor/Saving/BP_ControlSave.BP_ControlSave_C"))
      (return _returnvalue_3))))

(fn `SaveUserMapping`
  (params (MappingContext :type "InputMappingContext Object Reference") (Action :type "InputAction Object Reference") (NewKey :type "Key Structure" :default "None"))
  (`|ExecutionSequence`
    (:`then_0`
      (`|ExecutionSequence`
        (:`then_0`
          (set `/Game/InputPrompts/ManagerActor/Saving/BP_ControlSave.ContainsAlteredMappings` true (`self.SavedControls`)))
        (:`then_1`
          (for (_array_element _array_index) (`/Game/InputPrompts/ManagerActor/Saving/BP_ControlSave.SavedMappings` (`self.SavedControls`))
            (bind (_mappingcontext _action _mappedkey) (break `/Game/InputPrompts/ManagerActor/Saving/SavedMapping` _array_element))
            (if (and (== _mappingcontext (`local.MappingContext`)) (== _action (`local.Action`)) (== (`KismetInputLibrary.Key_IsGamepadKey` _mappedkey) (`KismetInputLibrary.Key_IsGamepadKey` (`local.NewKey`))))
              (`KismetArrayLibrary.Array_Remove` (`/Game/InputPrompts/ManagerActor/Saving/BP_ControlSave.SavedMappings` (`self.SavedControls`)) _array_index))))
        (:`then_2`
          (`KismetArrayLibrary.Array_Add` (`/Game/InputPrompts/ManagerActor/Saving/BP_ControlSave.SavedMappings` (`self.SavedControls`)) (make `/Game/InputPrompts/ManagerActor/Saving/SavedMapping` (`local.MappingContext`) (`local.Action`) (`local.NewKey`))))))
    (:`then_1`
      (`GameplayStatics.SaveGameToSlot` (`self.SavedControls`) (`self.SaveName`)))))