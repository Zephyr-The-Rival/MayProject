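; BP_TargetBounds is a volume actor that keeps spawning BP_FlyingTarget actors at random points inside its bounds.
; A Delay on Tick throttles the check to roughly every five seconds, spawning one target while the world holds fewer than twenty.
; Each random point within the Volume's box extents gets a zero-length sphere trace on Visibility, and spawning is skipped if it hits anything.
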(event `self.ReceiveTick`
  (params (DeltaSeconds :type "Float (single-precision)"))
  (`KismetSystemLibrary.Delay` 5.0)
  (bind _outactors (`GameplayStatics.GetAllActorsOfClass` "/Game/GrappleContent/Code/Target/BP_FlyingTarget.BP_FlyingTarget_C"))
  (if (< (`KismetArrayLibrary.Array_Length` _outactors) 20)
    (`self.SpawnTargetAtRandomLocation`)))

(fn `SpawnTargetAtRandomLocation`
  (bind _volume (`self.Volume`))
  (bind _locationtospawnat (`self.LocationToSpawnAt`))
  (bind _x (.x (`BoxComponent.GetScaledBoxExtent` _volume)))
  (bind _y (.y (`BoxComponent.GetScaledBoxExtent` _volume)))
  (bind _z (.z (`BoxComponent.GetScaledBoxExtent` _volume)))
  (set `self.LocationToSpawnAt` (+ (`SceneComponent.K2_GetComponentLocation` _volume) (`KismetMathLibrary.MakeVector` (`KismetMathLibrary.RandomFloatInRange` (* _x -1.0) _x) (`KismetMathLibrary.RandomFloatInRange` (* _y -1.0) _y) (`KismetMathLibrary.RandomFloatInRange` (* _z -1.0) _z))))
  (bind (_outhit _returnvalue) (`KismetSystemLibrary.SphereTraceSingle` _locationtospawnat _locationtospawnat 50.0 "TraceTypeQuery1"))
  (if (not _returnvalue)
    (`|SpawnActorFromClass` "/Game/GrappleContent/Code/Target/BP_FlyingTarget.BP_FlyingTarget_C" (`KismetMathLibrary.MakeTransform` (`self.LocationToSpawnAt`)) "Undefined" "MultiplyWithRoot" null null)))

(fn `UserConstructionScript`)