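; BP_Revolver is the player's revolver actor, handling the weapon's drum, reload props and electric firing effects.
; RotateDrum uses a timeline to roll the drum one 60-degree step from its current angle.
; Reload events spawn a speed loader in the player's left-hand socket, move the bullet mesh between loader and drum, and destroy the loader.
; OnShoot spawns railgun electricity Niagara arcs between random upper and lower gun sockets and pulses a point light.
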(event `RotateDrum`
  (set `self.DrumRollValue` (.roll (`SceneComponent.RelativeRotation` (`self.RevolverDrum`))))
  (bind (_direction _0_to_1) (`Timeline|Rotate` :!via `PlayFromStart`)
    (:`Update`
      (`SceneComponent.K2_SetRelativeRotation` (`self.RevolverDrum`) (`KismetMathLibrary.MakeRotator` (+ (* _0_to_1 60.0) (`self.DrumRollValue`))) false false))))

(event `SpawnSpeedLoader`
  (bind _speedloader (`self.SpeedLoader`))
  (bind _skeletalmeshcomponent (`SkeletalMeshActor.SkeletalMeshComponent` _speedloader))
  ;[1 1 1] Reload Evetns
  (bind _returnvalue (`|SpawnActorFromClass` "/Script/Engine.SkeletalMeshActor" (`KismetMathLibrary.MakeTransform` (0.0 0.0 0.0)) "Undefined" "MultiplyWithRoot" null null))
  (set `self.SpeedLoader` _returnvalue)
  (`SkeletalMeshComponent.SetSkeletalMeshAsset` _skeletalmeshcomponent "/Game/GrappleContent/Assets/Guns/Revolver/RevolverSpeedLoader.RevolverSpeedLoader")
  (`PrimitiveComponent.SetCollisionEnabled` _skeletalmeshcomponent "NoCollision")
  (`PrimitiveComponent.SetCastShadow` _skeletalmeshcomponent false)
  (bind _asbp_grapple_player_character (cast `/Game/GrappleContent/Code/PlayerAndGm/BP_GrapplePlayerCharacter` (`self.GetAttachParentActor`)))
  (`self.K2_AttachToComponent` _speedloader (`Character.Mesh` _asbp_grapple_player_character) "weapon_lSocket" "SnapToTarget" "SnapToTarget" "SnapToTarget" false)
  (`SceneComponent.K2_AttachToComponent` (`self.BulletMesh`) (`SkeletalMeshActor.SkeletalMeshComponent` (`self.SpeedLoader`)) "BulletsSocket" "SnapToTarget" "SnapToTarget" "SnapToTarget" true))

(event `AttachBulletsToGun`
  ;[1 1 1] Reload Evetns
  (`SceneComponent.K2_AttachToComponent` (`self.BulletMesh`) (`self.RevolverDrum`) "BulletSocket" "SnapToTarget" "SnapToTarget" "SnapToTarget" true))

(event `DestroySpeedLoader`
  ;[1 1 1] Reload Evetns
  (`self.K2_DestroyActor` (`self.SpeedLoader`)))

(event `self.OnShoot`
  (`|ExecutionSequence`
    (:`then_0`
      (`|ExecutionSequence`
        (:`then_0`
          (for _ (range 7)
            (bind _returnvalue (`NiagaraFunctionLibrary.SpawnSystemAttached` "/Game/GrappleContent/Assets/ParticleEffects/RailgunElectricity.RailgunElectricity" (`self.GunMesh`) "None" (0.0 0.0 0.0) (struct) "SnapToTarget"))
            (`|ExecutionSequence`
              (:`then_0`
                (`NiagaraComponent.SetVariableVec3` _returnvalue "Beam_Start" (.location (`SceneComponent.GetSocketTransform` (`self.GunMesh`) (`KismetSystemLibrary.MakeLiteralName` (`KismetStringLibrary.Conv_StringToName` (`KismetStringLibrary.Concat_StrStr` "ArcSocket_Up_" (`KismetStringLibrary.Conv_IntToString` (`KismetMathLibrary.RandomIntegerInRange` 0 11))))) "RTS_Component"))))
              (:`then_1`
                (`NiagaraComponent.SetVariableVec3` _returnvalue "End" (.location (`SceneComponent.GetSocketTransform` (`self.GunMesh`) (`KismetSystemLibrary.MakeLiteralName` (`KismetStringLibrary.Conv_StringToName` (`KismetStringLibrary.Concat_StrStr` "ArcSocket_Down_" (`KismetStringLibrary.Conv_IntToString` (`KismetMathLibrary.RandomIntegerInRange` 0 11))))) "RTS_Component")))))))
        (:`then_1`
          (bind (_direction _0___1__0) (`Timeline|Light Up` :!via `PlayFromStart`)
            (:`Update`
              (`LightComponent.SetIntensity` (`self.PointLight`) (* _0___1__0 50.0)))))))))

(fn `UserConstructionScript`)