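; BP_Door is a sliding double door that opens once when the grapple player character walks into its trigger box.
; The overlap calls Open, which destroys the box so it cannot fire again and plays a timeline.
; The timeline slides the Right and Left panels apart along Y in mirrored directions at a fixed height.
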(event `self.Box.OnComponentBeginOverlap`
  (params (OverlappedComponent :type "PrimitiveComponent Object Reference") (OtherActor :type "Actor Object Reference") (OtherComp :type "PrimitiveComponent Object Reference") (OtherBodyIndex :type Integer) (bFromSweep :type Boolean) (SweepResult :type "HitResult Structure (by ref)"))
  (cast `/Game/GrappleContent/Code/PlayerAndGm/BP_GrapplePlayerCharacter` OtherActor)
  (`self.Open`))

(event `Open`
  (`ActorComponent.K2_DestroyComponent` (`self.Box`))
  (bind (_direction _300_to__900) (`Timeline|Timeline` :!via `PlayFromStart`)
    (:`Update`
      (`SceneComponent.K2_SetRelativeLocation` (`self.Right`) (`KismetMathLibrary.MakeVector` 0.0 _300_to__900 900.0) false false)
      (`SceneComponent.K2_SetRelativeLocation` (`self.Left`) (`KismetMathLibrary.MakeVector` 0.0 (* _300_to__900 -1.0) 900.0) false false))))

(fn `UserConstructionScript`)