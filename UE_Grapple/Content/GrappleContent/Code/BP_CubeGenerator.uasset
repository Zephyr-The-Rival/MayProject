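; BP_CubeGenerator is a procedural scatter actor that fills a box, sized by the actor's scale, with randomly scaled cube meshes.
; When Active, its construction script adds NumCubes mesh components, then scales and offsets each around the root using RandomNegate for sign.
; Buildings mode uses a separate maximum height and sets Z to half-height, standing cubes on world zero.
; Unseeded randomness gives a new layout on every construction run.
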(fn `random negate`
  (params (a :type "Float (double-precision)"))
  (returns (`return value` :type "Float (double-precision)"))
  (if (`KismetMathLibrary.RandomBool`)
    (bind _result (`/Engine/EditorBlueprintResources/StandardMacros.NegateFloat` a)
      (:`  `
        (return _result)))
    (else
      (return a))))

(fn `UserConstructionScript`
  (bind (_returnvalue_x _returnvalue_y) (`KismetMathLibrary.BreakVector` (`SceneComponent.K2_GetComponentScale` (`self.Box`))))
  (bind (_returnvalue_x_2 _returnvalue_y_2 _returnvalue_z) (`KismetMathLibrary.BreakVector` (`SceneComponent.K2_GetComponentScale` (`self.Box`))))
  (`|ExecutionSequence`
    (:`then_0`
      (`KismetArrayLibrary.Array_Clear` (`self.Cubes`))
      (`KismetArrayLibrary.Array_Clear` (`self.Scales`)))
    (:`then_1`
      (if (`self.Active`)
        (`SceneComponent.SetWorldScale3D` (`self.Box`) (`self.GetActorScale3D`))
        (`|ExecutionSequence`
          (:`then_0`
            (for _ (range (`self.NumCubes`))
              (`|ExecutionSequence`
                (:`then_0`
                  (bind _returnvalue (`AddComponent|NODE_AddStaticMeshComponent-0`))
                  (`KismetArrayLibrary.Array_Add` (`self.Cubes`) _returnvalue))
                (:`then_1`
                  (if (`self.Buildings`)
                    (`KismetArrayLibrary.Array_Add` (`self.Scales`) (`KismetMathLibrary.MakeVector` (`KismetMathLibrary.RandomFloatInRange` (`self.MinScale`) (`self.MaxScale`)) (`KismetMathLibrary.RandomFloatInRange` (`self.MinScale`) (`self.MaxScale`)) (`KismetMathLibrary.RandomFloatInRange` (`self.MinScale`) (`self.MaxBuildingScale`))))
                    (else
                      (`KismetArrayLibrary.Array_Add` (`self.Scales`) (`KismetMathLibrary.MakeVector` (`KismetMathLibrary.RandomFloatInRange` (`self.MinScale`) (`self.MaxScale`)) (`KismetMathLibrary.RandomFloatInRange` (`self.MinScale`) (`self.MaxScale`)) (`KismetMathLibrary.RandomFloatInRange` (`self.MinScale`) (`self.MaxScale`))))))))))
          (:`then_1`
            (for (_array_element _array_index) (`self.Cubes`)
              (bind _output (`|GetArrayItem` (`self.Scales`) _array_index))
              (`SceneComponent.SetWorldScale3D` _array_element _output)
              (if (`self.Buildings`)
                (`SceneComponent.K2_SetWorldLocation` _array_element (`KismetMathLibrary.MakeVector` (.x (+ (`SceneComponent.K2_GetComponentLocation` (`self.DefaultSceneRoot`)) (* (`KismetMathLibrary.MakeVector` (`self.random negate` (`KismetMathLibrary.RandomFloatInRange` 0.0 _returnvalue_x)) (`self.random negate` (`KismetMathLibrary.RandomFloatInRange` 0.0 _returnvalue_y))) (50.0 50.0 1.0)))) (.y (+ (`SceneComponent.K2_GetComponentLocation` (`self.DefaultSceneRoot`)) (* (`KismetMathLibrary.MakeVector` (`self.random negate` (`KismetMathLibrary.RandomFloatInRange` 0.0 _returnvalue_x)) (`self.random negate` (`KismetMathLibrary.RandomFloatInRange` 0.0 _returnvalue_y))) (50.0 50.0 1.0)))) (* (.z _output) 50.0)) false false)
                (else
                  (`SceneComponent.K2_SetWorldLocation` _array_element (+ (`SceneComponent.K2_GetComponentLocation` (`self.DefaultSceneRoot`)) (* (`KismetMathLibrary.MakeVector` (`self.random negate` (`KismetMathLibrary.RandomFloatInRange` 0.0 _returnvalue_x_2)) (`self.random negate` (`KismetMathLibrary.RandomFloatInRange` 0.0 _returnvalue_y_2)) (`self.random negate` (`KismetMathLibrary.RandomFloatInRange` 0.0 _returnvalue_z))) (50.0 50.0 50.0))) false false))))))))))