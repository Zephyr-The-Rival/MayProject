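; First-person grapple player character that layers animation and visual feedback over its parent class's gun, grapple and wallrun states.
; State-change events play gun and grapple montages, using montage length to chain into the pull loop and time the grapple shooter's soft-cooldown end.
; Timelines roll the mesh into and out of wallrun tilts.
; Tick traces from the camera to flag grapple range and positions speed clouds along velocity, showing them at high speed.
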(event `self.ReceiveBeginPlay`)

(event `self.Wallrun_TiltMeshToSide`
  (params (bRight :type Boolean))
  (bind (_relativerotation_roll _relativerotation_pitch) (`KismetMathLibrary.BreakRotator` (`SceneComponent.RelativeRotation` (`self.Mesh`))))
  ;[1 1 1] Tilt For Wallrunning
  (set `self.Wallrunning` true)
  (set `self.Wallrunning_Right` bRight)
  (bind (_direction _0_to_1) (`Timeline|Timeline` :!via `PlayFromStart`)
    (:`Update`
      (if bRight
        (bind _returnvalue (* _0_to_1 (`self.WallrunTiltAngle`)))
        (`SceneComponent.K2_SetRelativeRotation` (`self.Mesh`) (`KismetMathLibrary.MakeRotator` (* _returnvalue -1.0) _relativerotation_pitch) false false)
        (else
          (`SceneComponent.K2_SetRelativeRotation` (`self.Mesh`) (`KismetMathLibrary.MakeRotator` _returnvalue _relativerotation_pitch) false false))))))

(event `self.OnGunStateChanged`
  (params (newState :type "EGunState Enum" :default "Idle"))
  ;[1 0.175 0.8996] Gun Animation Triggers
  (`parent.OnGunStateChanged` newState)
  (switch `EGunState` newState
    (:`Shooting`
      (`self.PlayAnimMontage` "/Game/GrappleContent/Assets/PlayerHands/Animations/Revolver/Shooting/Revolver_Shooting_Montage.Revolver_Shooting_Montage")
      (`|PlayMontage` (`Gun.GunMesh` (`self.CurrentGun`)) "/Game/GrappleContent/Assets/Guns/Revolver/Animations/Revolver_Shooting_Montage.Revolver_Shooting_Montage"))
    (:`Reloading`
      (`self.PlayAnimMontage` "/Game/GrappleContent/Assets/PlayerHands/Animations/Revolver/Shooting/FirstPerson_Revolver_Reloading_Montage.FirstPerson_Revolver_Reloading_Montage")
      (`|PlayMontage` (`Gun.GunMesh` (`self.CurrentGun`)) "/Game/GrappleContent/Assets/Guns/Revolver/Animations/Revolver_Reload_Montage.Revolver_Reload_Montage"))))

(event `self.Wallrun_TiltMeshBack`
  (bind _relativerotation_roll (`KismetMathLibrary.BreakRotator` (`SceneComponent.RelativeRotation` (`self.Mesh`))))
  (bind (_relativerotation_roll_2 _relativerotation_pitch) (`KismetMathLibrary.BreakRotator` (`SceneComponent.RelativeRotation` (`self.Mesh`))))
  ;[1 1 1] Tilt For Wallrunning
  (set `self.Wallrunning` false)
  (set `self.WallrunPreTiltBackValue` _relativerotation_roll)
  (bind (_direction _1_to_0) (`Timeline|Timeline_0` :!via `PlayFromStart`)
    (:`Update`
      (`SceneComponent.K2_SetRelativeRotation` (`self.Mesh`) (`KismetMathLibrary.MakeRotator` (* (`self.WallrunPreTiltBackValue`) _1_to_0) _relativerotation_pitch) false false))))

(event `self.OnGrappleStateChanged`
  (params (NewState :type "EGrappleState Enum" :default "Standby"))
  (`parent.OnGrappleStateChanged` NewState)
  (switch `EGrappleState` NewState
    (:`ShootingOut`
      (`self.PlayAnimMontage` "/Game/GrappleContent/Assets/PlayerHands/Animations/Grapple/FirstPerson_Grapple_ShootStart_Anim_Montage.FirstPerson_Grapple_ShootStart_Anim_Montage")
      (`KismetSystemLibrary.K2_PauseTimerHandle` (`self.SoftCooldownTimer`)))
    (:`Pulling`
      (bind _returnvalue (`self.PlayAnimMontage` "/Game/GrappleContent/Assets/PlayerHands/Animations/Grapple/FirstPerson_Grapple_PullStart_Anim_Montage.FirstPerson_Grapple_PullStart_Anim_Montage"))
      (`KismetSystemLibrary.Delay` _returnvalue)
      (if (`|EnumEquality` (`GrappleShooter.GetGrappleState` (`self.MyGrappleShooter`)) "Pulling")
        (`self.PlayAnimMontage` "/Game/GrappleContent/Assets/PlayerHands/Animations/Grapple/FirstPerson_Grapple_PullLoop_Montage.FirstPerson_Grapple_PullLoop_Montage")))
    (:`ReelingIn`
      (`self.PlayAnimMontage` "/Game/GrappleContent/Assets/PlayerHands/Animations/Grapple/FirstPerson_Grapple_ReelingIn_Montage.FirstPerson_Grapple_ReelingIn_Montage"))
    (:`CoolDown`
      (`self.PlayAnimMontage` "/Game/GrappleContent/Assets/PlayerHands/Animations/Grapple/FirstPerson_Grapple_CoolDown_Anim_Montage.FirstPerson_Grapple_CoolDown_Anim_Montage"))
    (:`SoftCoolDown`
      (bind _returnvalue_2 (`self.PlayAnimMontage` "/Game/GrappleContent/Assets/PlayerHands/Animations/Grapple/FirstPerson_Grapple_SoftCoolDown_Anim_Montage.FirstPerson_Grapple_SoftCoolDown_Anim_Montage"))
      (bind _returnvalue_3 (`KismetSystemLibrary.K2_SetTimerDelegate` (delegate `SoftCooldownOver`) _returnvalue_2))
      (set `self.SoftCooldownTimer` _returnvalue_3))))

(event `self.ReceiveTick`
  (params (DeltaSeconds :type "Float (single-precision)"))
  (bind _speedclouds (`self.SpeedClouds`))
  (bind _returnvalue (`SceneComponent.K2_GetComponentLocation` (`self.Camera`)))
  (bind _velocity (`MovementComponent.Velocity` (`self.CharacterMovementComponent`)))
  (`|ExecutionSequence`
    (:`then_0`
      ;[1 0 0] Check if grapple is in range
      (bind (_outhit _returnvalue_2) (`KismetSystemLibrary.LineTraceSingle` _returnvalue (+ _returnvalue (* (`SceneComponent.GetForwardVector` (`self.Camera`)) (`GrappleShooter.Range` (`self.MyGrappleShooter`)))) "TraceTypeQuery1"))
      (set `self.GrappleInRange` _returnvalue_2))
    (:`then_1`
      ;[1 0 0] Position Speed Clouds
      (`SceneComponent.K2_SetWorldLocation` _speedclouds (+ (`self.K2_GetActorLocation`) _velocity) false false)
      (`SceneComponent.SetVisibility` _speedclouds (> (`KismetMathLibrary.VSize` _velocity) 1500.0) false))))

(event `SoftCooldownOver`
  (`GrappleShooter.SoftCooldownOver` (`self.MyGrappleShooter`)))

(fn `UserConstructionScript`)